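; BP_T_Arrow is a one-shot trigger, likely a tutorial waypoint, that updates the UI when the player character overlaps its Box.
; Normally it displays its Text in the UI through PlayerControllerSiim, shows or hides the minimap per ShowMinimap, then destroys itself.
; When IsLast is set, it instead shows the main menu, destroys itself and resets PointsTotal in GameInstanceSiim.
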(event OnComponentBeginOverlap(Box)
  (params (OverlappedComponent :type Primitive%20Component%20Object%20Reference) (OtherActor :type Actor%20Object%20Reference) (OtherComp :type Primitive%20Component%20Object%20Reference) (OtherBodyIndex :type Integer) (bFromSweep :type Boolean) (SweepResult :type Hit%20Result%20Structure%20%28by%20ref%29))
  (Utilities|Casting|CastToBP_ThirdPersonCharacter_Siim OtherActor)
  (bind _asplayer_controller_siim (Utilities|Casting|CastToPlayerControllerSiim (Game|GetPlayerController 0)))
  (if (Variables|Default|GetIsLast?)
    (Widget|SetVisibility (Variables|/Game/Siim/UI/UI_Main.UI_Main_C|GetUI_MainMenu (Variables|/Game/Siim/PlayerControllerSiim.PlayerControllerSiim_C|GetUI_Main _asplayer_controller_siim)) "Visible")
    (Actor|DestroyActor)
    (bind _asgame_instance_siim (Utilities|Casting|CastToGameInstanceSiim (Game|GetGameInstance)))
    (Variables|/Game/Siim/GameInstanceSiim.GameInstanceSiim_C|SetPointsTotal _asgame_instance_siim 0.0)
    (else
      (Variables|/Game/Siim/UI/UI_Text.UI_Text_C|SetTextText (Variables|/Game/Siim/UI/UI_Main.UI_Main_C|GetUI_Text (Variables|/Game/Siim/PlayerControllerSiim.PlayerControllerSiim_C|GetUI_Main _asplayer_controller_siim)) (Variables|Default|GetText))
      (Widget|SetVisibility (Variables|/Game/Siim/UI/UI_Main.UI_Main_C|GetUI_Text (Variables|/Game/Siim/PlayerControllerSiim.PlayerControllerSiim_C|GetUI_Main _asplayer_controller_siim)) "Visible")
      (if (Variables|Default|GetShowMinimap)
        (Widget|SetVisibility (Variables|/Game/Siim/UI/UI_Main.UI_Main_C|GetUI_Minimap (Variables|/Game/Siim/PlayerControllerSiim.PlayerControllerSiim_C|GetUI_Main _asplayer_controller_siim)) "Visible")
        (Actor|DestroyActor)
        (else
          (Widget|SetVisibility (Variables|/Game/Siim/UI/UI_Main.UI_Main_C|GetUI_Minimap (Variables|/Game/Siim/PlayerControllerSiim.PlayerControllerSiim_C|GetUI_Main _asplayer_controller_siim)) "Hidden")
          (Actor|DestroyActor))))))

(fn ConstructionScript)