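; BP_TaskUI is a 3D minimap of the correct cube path, with scene captures for front, side and top views.
; It builds scaled-down static meshes from RoomManager's CorrectCubeLocations on start and on CoordinatesGenerated, marking first, last and current cubes.
; Each capture is offset by half the first-to-last span to center the path.
; ShowCharacterLocation advances the current-cube marker one step along the path.
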(event Custom|Create3DforMap
  (bind _roommanager (Variables|Default|GetRoomManager))
  (bind _dimfactor (Variables|Default|GetDimFactor))
  (bind _scenecapture_01_front (Variables|Default|GetSceneCapture_01_Front))
  (bind _scenecapture_02_side (Variables|Default|GetSceneCapture_02_Side))
  (bind _scenecapture_03_top (Variables|Default|GetSceneCapture_03_Top))
  (bind _roommanager_2 (Variables|Default|GetRoomManager))
  (bind _relativelocation (Variables|/Script/Engine.SceneComponent|GetRelativeLocation _scenecapture_03_top))
  (bind _correctcubelocations (Variables|/Game/Siim/BP_RoomManager.BP_RoomManager_C|GetCorrectCubeLocations _roommanager))
  (bind _relativelocation_2 (Variables|/Script/Engine.SceneComponent|GetRelativeLocation _scenecapture_01_front))
  (bind _relativelocation_3 (Variables|/Script/Engine.SceneComponent|GetRelativeLocation _scenecapture_02_side))
  (bind _correctcubelocations_2 (Variables|/Game/Siim/BP_RoomManager.BP_RoomManager_C|GetCorrectCubeLocations _roommanager_2))
  (bind _returnvalue (Utilities|Array|LastIndex _correctcubelocations))
  (bind _output (Utilities|Array|Get(acopy) _correctcubelocations))
  (bind _output_2 (Utilities|Array|Get(acopy) _correctcubelocations _returnvalue))
  (bind _returnvalue_2 (- _output_2 _output))
  (bind _returnvalue_3 (/ _returnvalue_2 _dimfactor))
  (bind _returnvalue_4 (/ (.x _returnvalue_3) 2.0))
  (bind _returnvalue_5 (/ (.z _returnvalue_3) 2.0))
  (bind _returnvalue_6 (/ (.y _returnvalue_3) 2.0))
  ;[1 1 1] CREATE Cube Formation according to placement
  (for (_array_element _array_index) _correctcubelocations_2
    (bind _returnvalue_7 (AddComponent|AddStaticMeshComponent false (Math|Transform|MakeTransform (/ _array_element (Variables|Default|GetDimFactor)) "0, 0, 0" "1.000000,1.000000,1.000000")))
    (if (== _array_index 0)
      (Components|StaticMesh|SetStaticMesh _returnvalue_7 "/Game/Siim/SM/MinimapCube_First.MinimapCube_First")
      ;[1 1 1] Places Correct Cube marker (Red) to Minimap (1st cube)
      (bind _returnvalue_8 (AddComponent|AddStaticMeshComponent false (Math|Transform|MakeTransform (/ _array_element (Variables|Default|GetDimFactor)) "0, 0, 0" "1.500000,1.500000,1.500000")))
      (bind _output_get (Variables|Default|SetSM_LocIndicator _returnvalue_8))
      (Components|StaticMesh|SetStaticMesh _output_get "/Game/Siim/SM/MinimapCube_Current.MinimapCube_Current")
      (elif (== _array_index (- (Utilities|Array|Length _correctcubelocations_2) 1))
        (Components|StaticMesh|SetStaticMesh _returnvalue_7 "/Game/Siim/SM/MinimapCube_Last.MinimapCube_Last")
        (else
          (Components|StaticMesh|SetStaticMesh _returnvalue_7 "/Game/Siim/SM/MinimapCube.MinimapCube")))))
  ;[1 1 1] Make sure the camera is centered (and aligned) in all 3 views
  (Transformation|SetRelativeLocation _scenecapture_01_front (Math|Vector|MakeVector (.x _relativelocation_2) (+ (.y _relativelocation_2) _returnvalue_6) (+ (.z _relativelocation_2) _returnvalue_5)) false false)
  (Transformation|SetRelativeLocation _scenecapture_02_side (Math|Vector|MakeVector (+ (.x _relativelocation_3) _returnvalue_4) (.y _relativelocation_3) (+ (.z _relativelocation_3) _returnvalue_5)) false false)
  (Transformation|SetRelativeLocation _scenecapture_03_top (Math|Vector|MakeVector (+ (.x _relativelocation) _returnvalue_4) (+ (.y _relativelocation) _returnvalue_6) (+ (.z _relativelocation) _returnvalue_5)) false false))

(event Custom|ShowCharacterLocation
  ;[1 1 1] Sets new location on MiniMap
  (bind _output_get (Variables|Default|SetCorrectCubeindex (+ 1 (Variables|Default|GetCorrectCubeindex))))
  (Transformation|SetRelativeLocation (Variables|Default|GetSM_LocIndicator) (/ (Utilities|Array|Get(acopy) (Variables|/Game/Siim/BP_RoomManager.BP_RoomManager_C|GetCorrectCubeLocations (Variables|Default|GetRoomManager)) _output_get) (Variables|Default|GetDimFactor)) false false))

(event EventBeginPlay
  (Utilities|FlowControl|Delay 0.2)
  (bind _asbp_third_person_character_siim (Utilities|Casting|CastToBP_ThirdPersonCharacter_Siim (Game|GetPlayerCharacter 0)))
  (bind _output_get (Variables|Default|SetAs%20BP%20Third%20Person%20Character%20Siim _asbp_third_person_character_siim))
  (EventDispatchers|BindEventtoPlayerBeginOverlapCorrectCollision _output_get (EventDispatchers|CreateEvent :!event Custom|ShowCharacterLocation))
  (bind _asgame_instance_siim (Utilities|Casting|CastToGameInstanceSiim (Game|GetGameInstance)))
  (bind _output_get_2 (Variables|Default|SetRoomManager (Variables|/Game/Siim/GameInstanceSiim.GameInstanceSiim_C|GetRoomManager _asgame_instance_siim)))
  (EventDispatchers|BindEventtoCoordinatesGenerated _output_get_2 (delegate Custom|Create3DforMap))
  (CallFunction|Create3DforMap)
  (EventDispatchers|BindEventtoPlayerBeginOverlapCorrectCollision (Variables|Default|GetAs%20BP%20Third%20Person%20Character%20Siim) (EventDispatchers|CreateEvent :!event Custom|ShowCharacterLocation)))

(fn ConstructionScript)