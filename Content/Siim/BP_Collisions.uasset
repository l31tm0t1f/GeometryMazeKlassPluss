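; Gameplay actor that spawns trigger boxes over the RoomManager's correct and death cubes and handles scoring and winning.
; It builds tagged box components at runtime from cube locations, skipping the first correct cube, and binds to player overlap events.
; Correct hits award time-based points and destroy their box, with the last in the array triggering the win UI.
; Death hits apply a points penalty and briefly show damage text.
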(event Custom|CreateCollisions
  (bind _correctcollisionsarray (Variables|Default|GetCorrectCollisionsArray))
  ;[1 1 1] Create Collisions (Correct and Death ones)
  ;;[1 1 1] Correct Collisions
  (for (_array_element _array_index) (Variables|/Game/Siim/BP_RoomManager.BP_RoomManager_C|GetCorrectCubeLocations (Variables|/Game/Siim/GameInstanceSiim.GameInstanceSiim_C|GetRoomManager (stale EventBeginPlay _asgame_instance_siim)))
    (if (!= _array_index 0)
      (bind _returnvalue (AddComponent|AddBoxComponent false (Math|Transform|MakeTransform (+ _array_element "0,0,300.000000") "0, 0, 0" "12.000000,12.000000,12.000000")))
      (Variables|/Script/Engine.ActorComponent|SetComponentTags _returnvalue (Variables|Default|GetCorrectCollisionsTags))
      (Utilities|Array|Add (Variables|Default|GetCorrectCollisionsArray) _returnvalue)))
  (Variables|Default|SetCorrectCollisionLast (Utilities|Array|Get(acopy) _correctcollisionsarray (Utilities|Array|LastIndex _correctcollisionsarray)))
  ;;[1 1 1] Death Collisions
  (for _array_element_2 (Variables|/Game/Siim/BP_RoomManager.BP_RoomManager_C|GetDeathCubeLocations (Variables|/Game/Siim/GameInstanceSiim.GameInstanceSiim_C|GetRoomManager (stale EventBeginPlay _asgame_instance_siim)))
    (bind _returnvalue_2 (AddComponent|AddBoxComponent false (Math|Transform|MakeTransform (+ _array_element_2 "0,0,300.000000") "0, 0, 0" "12.000000,12.000000,12.000000")))
    (Variables|/Script/Engine.ActorComponent|SetComponentTags _returnvalue_2 (Variables|Default|GetDeathCollisionsTags))
    (Utilities|Array|Add (Variables|Default|GetDeathCollisionsArray) _returnvalue_2)))

(event Custom|CollidesWithCorrectCollision
  (bind _elapsedtime_0 (Variables|Default|GetElapsedTime_0))
  (bind _pointsmin (Variables|Default|GetPointsMin))
  ;[1 1 1] Going to the right Cube - add points
  (bind _asgame_instance_siim (Utilities|Casting|CastToGameInstanceSiim (Game|GetGameInstance)))
  (if (< (Variables|Default|GetElapsedTime) _elapsedtime_0)
    (Variables|/Game/Siim/GameInstanceSiim.GameInstanceSiim_C|SetPointsAdd _asgame_instance_siim (Math|Conversions|ToFloat(Integer) (Math|Float|Round (+ (* 5.0 (- _elapsedtime_0 (Variables|Default|GetElapsedTime))) _pointsmin)))) ; ADDED POINTS
    (bind _asplayer_controller_siim (Utilities|Casting|CastToPlayerControllerSiim (Game|GetPlayerController 0)))
    (Widget|SetVisibility (Variables|/Game/Siim/UI/UI_Main.UI_Main_C|GetUI_PointsAdd (Variables|/Game/Siim/PlayerControllerSiim.PlayerControllerSiim_C|GetUI_Main _asplayer_controller_siim)) "Visible")
    (Variables|/Game/Siim/GameInstanceSiim.GameInstanceSiim_C|SetPointsTotal _asgame_instance_siim (Math|Conversions|ToFloat(Integer) (Math|Float|Round (+ (+ (* 5.0 (- _elapsedtime_0 (Variables|Default|GetElapsedTime))) _pointsmin) (Variables|/Game/Siim/GameInstanceSiim.GameInstanceSiim_C|GetPointsTotal _asgame_instance_siim))))) ; TOTAL POINTS
    (else
      (bind _output_get (Variables|/Game/Siim/GameInstanceSiim.GameInstanceSiim_C|SetPointsAdd _asgame_instance_siim _pointsmin)) ; ADDED POINTS
      (Variables|/Game/Siim/GameInstanceSiim.GameInstanceSiim_C|SetPointsTotal _asgame_instance_siim (+ (Variables|/Game/Siim/GameInstanceSiim.GameInstanceSiim_C|GetPointsTotal _asgame_instance_siim) _output_get)) ; TOTAL POINTS
    ))
  (Variables|Default|SetElapsedTime 0.0)
  ;[1 1 1] Destroy Collision
  (bind _asbp_third_person_character_siim (Utilities|Casting|CastToBP_ThirdPersonCharacter_Siim (Game|GetPlayerCharacter 0)))
  (Variables|Default|SetCompareWithThatCollision (Variables|/Game/Siim/BP_ThirdPersonCharacter_Siim.BP_ThirdPersonCharacter_Siim_C|GetDestroyThatCollision _asbp_third_person_character_siim))
  (Components|DestroyComponent (Variables|/Game/Siim/BP_ThirdPersonCharacter_Siim.BP_ThirdPersonCharacter_Siim_C|GetDestroyThatCollision _asbp_third_person_character_siim))
  ;[1 1 1] Last Collision - Winning COndition
  (if (== (Variables|Default|GetCompareWithThatCollision) (Variables|Default|GetCorrectCollisionLast))
    (bind _asplayer_controller_siim_2 (Utilities|Casting|CastToPlayerControllerSiim (Game|GetPlayerController 0)))
    (CallFunction|DisableInputandMovement)
    (Input|SetInputModeUIOnly _asplayer_controller_siim_2 0 "DoNotLock")
    (Variables|/Script/Engine.PlayerController|SetbShowMouseCursor _asplayer_controller_siim_2 true)
    (Variables|/Game/Siim/UI/UI_Text.UI_Text_C|SetTextText (Variables|/Game/Siim/UI/UI_Main.UI_Main_C|GetUI_Text (Variables|/Game/Siim/PlayerControllerSiim.PlayerControllerSiim_C|GetUI_Main _asplayer_controller_siim_2)) "You Won")
    (Widget|SetVisibility (Variables|/Game/Siim/UI/UI_Main.UI_Main_C|GetUI_Text (Variables|/Game/Siim/PlayerControllerSiim.PlayerControllerSiim_C|GetUI_Main _asplayer_controller_siim_2)) "Visible")
    (Utilities|FlowControl|Delay 3.0)
    (Widget|SetVisibility (Variables|/Game/Siim/UI/UI_Main.UI_Main_C|GetUI_Text (Variables|/Game/Siim/PlayerControllerSiim.PlayerControllerSiim_C|GetUI_Main _asplayer_controller_siim_2)) "Hidden")))

(event Custom|CollidesWithDeathCollision
  (bind _pointsdamage (Variables|Default|GetPointsDamage))
  ;[1 1 1] Going to the Death Cube - minus points or death
  (bind _asgame_instance_siim (Utilities|Casting|CastToGameInstanceSiim (Game|GetGameInstance)))
  (Variables|/Game/Siim/GameInstanceSiim.GameInstanceSiim_C|SetPointsAdd _asgame_instance_siim _pointsdamage)
  (bind _asplayer_controller_siim (Utilities|Casting|CastToPlayerControllerSiim (Game|GetPlayerController 0)))
  (Widget|SetVisibility (Variables|/Game/Siim/UI/UI_Main.UI_Main_C|GetCanvas_PointsAdd (Variables|/Game/Siim/PlayerControllerSiim.PlayerControllerSiim_C|GetUI_Main _asplayer_controller_siim)) "Visible")
  (Variables|/Game/Siim/GameInstanceSiim.GameInstanceSiim_C|SetPointsTotal _asgame_instance_siim (+ (Variables|/Game/Siim/GameInstanceSiim.GameInstanceSiim_C|GetPointsTotal _asgame_instance_siim) _pointsdamage))
  ;[1 1 1] Damage (Sound / Camera Wobble / Blood on UI)
  (bind _asplayer_controller_siim_2 (Utilities|Casting|CastToPlayerControllerSiim (Game|GetPlayerController 0)))
  (Variables|/Game/Siim/UI/UI_Text.UI_Text_C|SetTextText (Variables|/Game/Siim/UI/UI_Main.UI_Main_C|GetUI_Text (Variables|/Game/Siim/PlayerControllerSiim.PlayerControllerSiim_C|GetUI_Main _asplayer_controller_siim_2)) "Damage")
  (Widget|SetVisibility (Variables|/Game/Siim/UI/UI_Main.UI_Main_C|GetUI_Text (Variables|/Game/Siim/PlayerControllerSiim.PlayerControllerSiim_C|GetUI_Main _asplayer_controller_siim_2)) "Visible")
  (Utilities|FlowControl|Delay 5.0)
  (Widget|SetVisibility (Variables|/Game/Siim/UI/UI_Main.UI_Main_C|GetUI_Text (Variables|/Game/Siim/PlayerControllerSiim.PlayerControllerSiim_C|GetUI_Main _asplayer_controller_siim_2)) "Hidden"))

(event EventBeginPlay
  (Utilities|FlowControl|Delay 0.2)
  (bind _asgame_instance_siim (Utilities|Casting|CastToGameInstanceSiim (Game|GetGameInstance)))
  (bind _output_get (Variables|Default|SetRoom%20Manager (Variables|/Game/Siim/GameInstanceSiim.GameInstanceSiim_C|GetRoomManager _asgame_instance_siim)))
  (EventDispatchers|BindEventtoCoordinatesGenerated _output_get (EventDispatchers|CreateEvent :!event Custom|CreateCollisions))
  (Utilities|FlowControl|Delay 0.2)
  (CallFunction|CreateCollisions)
  (bind _asbp_third_person_character_siim (Utilities|Casting|CastToBP_ThirdPersonCharacter_Siim (Game|GetPlayerCharacter 0)))
  (EventDispatchers|BindEventtoPlayerBeginOverlapCorrectCollision _asbp_third_person_character_siim (EventDispatchers|CreateEvent :!event Custom|CollidesWithCorrectCollision))
  (EventDispatchers|BindEventtoPlayerBeginOverlapDeathCollision _asbp_third_person_character_siim (EventDispatchers|CreateEvent :!event Custom|CollidesWithDeathCollision)))

(event EventTick
  (params (DeltaSeconds :type Float%20%28single-precision%29))
  ;[1 1 1] Count seconds
  (Variables|Default|SetElapsedTime (+ DeltaSeconds (Variables|Default|GetElapsedTime))))

(fn ConstructionScript)