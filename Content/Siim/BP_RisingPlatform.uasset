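; Rising platform actor that carries the player one room step up or down through the cube-room grid.
; It builds a 3D grid of platform meshes with tagged collision boxes, sized and spaced from the RoomManager.
; Player overlap and Up-Down UI events drive the menu, input locking and movement.
; Timelines lerp the whole actor by one Z step, with a DoOnce that resets when overlap ends.
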(event Custom|GoesUpOrDown
  (params (IsUp :type Boolean))
  ;[1 1 1] UP-DOWN movement
  (bind _asgame_instance_siim (Utilities|Casting|CastToGameInstanceSiim (Game|GetGameInstance)))
  (Variables|Default|SetCurrentLocation (Transformation|GetActorLocation))
  (Utilities|FlowControl|DoOnce false
    (:Completed
      (|Level_Basic (Variables|/Game/Siim/GameInstanceSiim.GameInstanceSiim_C|GetRoomManager _asgame_instance_siim) IsUp))))

(event Custom|Create%20All%20Platforms
  ;[1 1 1] Create Platforms
  (bind _asgame_instance_siim (Utilities|Casting|CastToGameInstanceSiim (Game|GetGameInstance)))
  (bind _output_get (Variables|Default|SetFirstPlatformLocation (Math|Vector|MakeVector (* (Math|Conversions|ToFloat(Integer) (Variables|/Game/Siim/BP_RoomManager.BP_RoomManager_C|GetCubesOnOneSide (Variables|/Game/Siim/GameInstanceSiim.GameInstanceSiim_C|GetRoomManager _asgame_instance_siim))) (.x (Variables|/Game/Siim/BP_RoomManager.BP_RoomManager_C|GetStepXYZ (Variables|/Game/Siim/GameInstanceSiim.GameInstanceSiim_C|GetRoomManager _asgame_instance_siim))) -1.0) (* (Math|Conversions|ToFloat(Integer) (Variables|/Game/Siim/BP_RoomManager.BP_RoomManager_C|GetCubesOnOneSide (Variables|/Game/Siim/GameInstanceSiim.GameInstanceSiim_C|GetRoomManager _asgame_instance_siim))) (.y (Variables|/Game/Siim/BP_RoomManager.BP_RoomManager_C|GetStepXYZ (Variables|/Game/Siim/GameInstanceSiim.GameInstanceSiim_C|GetRoomManager _asgame_instance_siim))) -1.0) (* -1.0 (.z (Variables|/Game/Siim/BP_RoomManager.BP_RoomManager_C|GetStepXYZ (Variables|/Game/Siim/GameInstanceSiim.GameInstanceSiim_C|GetRoomManager _asgame_instance_siim)))))))
  ;;[1 1 1] Plaforms X-direction
  (for _index (range 0 (+ (Variables|/Game/Siim/BP_RoomManager.BP_RoomManager_C|GetCubesOnOneSide (Variables|/Game/Siim/GameInstanceSiim.GameInstanceSiim_C|GetRoomManager _asgame_instance_siim)) (Variables|/Game/Siim/BP_RoomManager.BP_RoomManager_C|GetCubesOnOneSide (Variables|/Game/Siim/GameInstanceSiim.GameInstanceSiim_C|GetRoomManager _asgame_instance_siim))))
    (bind _output_get_2 (Variables|Default|SetCurrentPlatformLocation (Math|Vector|MakeVector (+ (.x _output_get) (* _index (.x (Variables|/Game/Siim/BP_RoomManager.BP_RoomManager_C|GetStepXYZ (Variables|/Game/Siim/GameInstanceSiim.GameInstanceSiim_C|GetRoomManager _asgame_instance_siim))))) (.y _output_get) (.z _output_get))))
    (CallFunction|CreatePlatformWCollision (Math|Vector|MakeVector (.x _output_get_2) (.y _output_get_2) (.z _output_get_2)))
    ;;[1 1 1] Plaforms Y-direction
    (for _index_2 (range 0 (+ (Variables|/Game/Siim/BP_RoomManager.BP_RoomManager_C|GetCubesOnOneSide (Variables|/Game/Siim/GameInstanceSiim.GameInstanceSiim_C|GetRoomManager _asgame_instance_siim)) (Variables|/Game/Siim/BP_RoomManager.BP_RoomManager_C|GetCubesOnOneSide (Variables|/Game/Siim/GameInstanceSiim.GameInstanceSiim_C|GetRoomManager _asgame_instance_siim))))
      (bind _output_get_3 (Variables|Default|SetCurrentPlatformLocation (Math|Vector|MakeVector (.x _output_get_2) (+ (.y (Variables|Default|GetFirstPlatformLocation)) (* _index_2 (.y (Variables|/Game/Siim/BP_RoomManager.BP_RoomManager_C|GetStepXYZ (Variables|/Game/Siim/GameInstanceSiim.GameInstanceSiim_C|GetRoomManager _asgame_instance_siim))))) (.z _output_get_2))))
      (CallFunction|CreatePlatformWCollision _output_get_3)
      ;;[1 1 1] Plaforms Z-direction
      (for _index_3 (range 0 (+ (Variables|/Game/Siim/BP_RoomManager.BP_RoomManager_C|GetCubesOnOneSide (Variables|/Game/Siim/GameInstanceSiim.GameInstanceSiim_C|GetRoomManager _asgame_instance_siim)) (Variables|/Game/Siim/BP_RoomManager.BP_RoomManager_C|GetCubesOnOneSide (Variables|/Game/Siim/GameInstanceSiim.GameInstanceSiim_C|GetRoomManager _asgame_instance_siim))))
        (bind _output_get_4 (Variables|Default|SetCurrentPlatformLocation (Math|Vector|MakeVector (.x _output_get_2) (.y _output_get_2) (+ (.z (Variables|Default|GetFirstPlatformLocation)) (* _index_3 (.z (Variables|/Game/Siim/BP_RoomManager.BP_RoomManager_C|GetStepXYZ (Variables|/Game/Siim/GameInstanceSiim.GameInstanceSiim_C|GetRoomManager _asgame_instance_siim))))))))
        (CallFunction|CreatePlatformWCollision _output_get_4)))))

(event Custom|EndOverlap
  ;[1 1 1] UP-DOWN movement
  (CallFunction|EnableInputandMovement)
  (Utilities|FlowControl|DoOnce false) ; enters at Reset
)

(event Custom|ShowUpDownUI
  ;[1 1 1] Open Up-Down menu, disable outputs etc
  (bind _asplayer_controller_siim (Utilities|Casting|CastToPlayerControllerSiim (Game|GetPlayerController 0)))
  (Widget|SetVisibility (Variables|/Game/Siim/UI/UI_Main.UI_Main_C|GetUI_Up-Down (Variables|/Game/Siim/PlayerControllerSiim.PlayerControllerSiim_C|GetUI_Main _asplayer_controller_siim)) "Visible")
  (CallFunction|DisableInputandMovement))

(event EventBeginPlay
  ;[1 1 1] Comment
  (Utilities|FlowControl|Delay 0.2)
  (bind _asgame_instance_siim (Utilities|Casting|CastToGameInstanceSiim (Game|GetGameInstance)))
  (bind _output_get (Variables|Default|SetRoomManager (Variables|/Game/Siim/GameInstanceSiim.GameInstanceSiim_C|GetRoomManager _asgame_instance_siim)))
  (EventDispatchers|BindEventtoCoordinatesGenerated _output_get (EventDispatchers|CreateEvent :!event Custom|Create%20All%20Platforms))
  (CallFunction|CreateAllPlatforms)
  (bind _asplayer_controller_siim (Utilities|Casting|CastToPlayerControllerSiim (Game|GetPlayerController 0)))
  (EventDispatchers|BindEventtoUporDown (Variables|/Game/Siim/UI/UI_Main.UI_Main_C|GetUI_Up-Down (Variables|/Game/Siim/PlayerControllerSiim.PlayerControllerSiim_C|GetUI_Main _asplayer_controller_siim)) (EventDispatchers|CreateEvent :!event Custom|GoesUpOrDown))
  (bind _asbp_third_person_character_siim (Utilities|Casting|CastToBP_ThirdPersonCharacter_Siim (Game|GetPlayerCharacter 0)))
  (bind _output_get_2 (Variables|Default|SetPlayerCharacter _asbp_third_person_character_siim))
  (EventDispatchers|BindEventtoPlayerBeginOverlapPlatform _output_get_2 (EventDispatchers|CreateEvent :!event Custom|ShowUpDownUI))
  (EventDispatchers|BindEventtoPlayerEndOverlapPlatform _output_get_2 (EventDispatchers|CreateEvent :!event Custom|EndOverlap)))

(fn ConstructionScript)

(fn CreatePlatformWCollision
  (params (VectorLocation :type Vector))
  ;[1 1 1] Create Platform + Collision
  (bind _returnvalue (AddComponent|AddStaticMeshComponent false (Math|Transform|MakeTransform VectorLocation "0, 0, 0" "1.000000,1.000000,1.000000")))
  (Components|StaticMesh|SetStaticMesh _returnvalue "/Game/Siim/SM/Cube_parts_Mesh3.Cube_parts_Mesh3")
  (bind _returnvalue_2 (AddComponent|AddBoxComponent false (Math|Transform|MakeTransform VectorLocation "0, 0, 0" "0.050000,0.050000,3.000000")))
  (Variables|/Script/Engine.ActorComponent|SetComponentTags _returnvalue_2 (Variables|Default|GetTagArray)))